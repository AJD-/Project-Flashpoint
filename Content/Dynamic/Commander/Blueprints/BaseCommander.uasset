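; Base commander pawn that gives the player a mouse-and-axis driven camera with a visible cursor.
; Strafing follows the actor's right vector and the scroll wheel moves along the camera's view; ForwardHorizontal passes a zero direction, leaving its flattened-forward math unconnected.
; Holding middle mouse hides and recenters the cursor while turning and pitching, with pitch clamped back once it exceeds MaximumLookDirection.
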(event EventBeginPlay
  (Variables|/Script/Engine.PlayerController|SetbShowMouseCursor (Game|GetPlayerController 0) true))

(event Input|ActionEvents|InputActionMiddleMouse
  (params (Key :type Key%20Structure))
  (bind _returnvalue (Game|GetPlayerController 0))
  ;[1 1 1] Look Controlls
  (:Pressed
    (Variables|Default|SetMiddleMouse true)
    (Variables|/Script/Engine.PlayerController|SetbShowMouseCursor _returnvalue false))
  (:Released
    (Variables|Default|SetMiddleMouse false)
    (Variables|/Script/Engine.PlayerController|SetbShowMouseCursor _returnvalue true)))

(event Input|AxisEvents|InputAxisMoveForward
  (params (AxisValue :type Float%20%28single-precision%29))
  ;[1 1 1] Movement Controls
  (CallFunction|ForwardHorizontal AxisValue))

(event Input|AxisEvents|InputAxisMoveRight
  (params (AxisValue :type Float%20%28single-precision%29))
  ;[1 1 1] Movement Controls
  (Pawn|Input|AddMovementInput (Transformation|GetActorRightVector) AxisValue false))

(event Input|AxisEvents|InputAxisScrollWheel
  (params (AxisValue :type Float%20%28single-precision%29))
  ;[1 1 1] Look Controlls
  (Pawn|Input|AddMovementInput (Math|Vector|GetForwardVector (Variables|Default|GetCamera)) AxisValue false))

(event Input|AxisEvents|InputAxisTurn
  (params (AxisValue :type Float%20%28single-precision%29))
  ;[1 1 1] Look Controlls
  (if (Variables|Default|GetMiddleMouse)
    (Pawn|Input|AddControllerYawInput AxisValue)
    (CallFunction|RecenterCursor)))

(event Input|AxisEvents|InputAxisLookUp
  (params (AxisValue :type Float%20%28single-precision%29))
  (bind _camera (Variables|Default|GetCamera))
  (bind _returnvalue (Transformation|GetWorldRotation _camera))
  (bind (_roll _pitch _yaw) (Math|Rotator|BreakRotator _returnvalue))
  ;[1 1 1] Look Controlls
  (if (Variables|Default|GetMiddleMouse)
    (Math|Float|CompareFloat _pitch (+ (Variables|Default|GetMaximum%20Look%20Direction) 0.0001)
      (:>
        (Pawn|SetControlRotation (Game|GetPlayerController 0) (Math|Rotator|MakeRotator _roll (Math|Float|Clamp(Float) _pitch -9e+01 (Variables|Default|GetMaximum%20Look%20Direction)) _yaw)))
      (:==
        (Pawn|Input|AddControllerPitchInput AxisValue :!label _label))
      (:<
        (goto _label)))
    (CallFunction|RecenterCursor)))

(fn ConstructionScript)

(fn RecenterCursor
  (bind _returnvalue (Game|GetPlayerController 0))
  (bind _returnvalue_2 (Viewport|GetViewportSize))
  (bind (_x _y) (Math|Vector2D|BreakVector2D _returnvalue_2))
  (if (not (Variables|/Script/Engine.PlayerController|GetbShowMouseCursor _returnvalue))
    (Class|PlayerController|SetMouseLocation _returnvalue (Math|Float|Truncate (/ _x 2.0)) (Math|Float|Truncate (/ _y 2.0)))))

(fn ForwardHorizontal
  (params (ScaleValue :type Float%20%28single-precision%29))
  (Pawn|Input|AddMovementInput "0, 0, 0" ScaleValue false))