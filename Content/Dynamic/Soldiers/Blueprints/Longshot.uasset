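; Longshot soldier Blueprint whose Aim input drives a scoped aiming mode and only allows firing while aiming.
; A timeline plays and reverses to blend camera FOV and PlayerHUD scope opacity, printing the opacity each update as debug output.
; Aiming scales walk speed down and release multiplies it back, routed through a server event to a multicast.
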(event Custom|Server%20Modify%20Movement%20Speed
  (params (newSpeed :type Float%20%28single-precision%29))
  (CallFunction|MulticastModifyMovementSpeed newSpeed))

(event Custom|Multicast%20Modify%20Movement%20Speed
  (params (newSpeed :type Float%20%28single-precision%29))
  (Variables|/Script/Engine.CharacterMovementComponent|SetMaxWalkSpeed (Variables|Character|GetCharacterMovement) newSpeed))

(event EventBeginPlay
  (|CallParentFunction))

(event Collision|EventActorBeginOverlap
  (params (OtherActor :type Actor%20Object%20Reference)))

(event EventTick
  (params (DeltaSeconds :type Float%20%28single-precision%29))
  (|CallParentFunction DeltaSeconds) ; This node is disabled and will not be called.\nDrag off pins to build functionality.
)

(event Input|ActionEvents|InputActionAim
  (params (Key :type Key%20Structure))
  (bind _fire (Variables|Default|GetFire))
  (bind _charactermovement (Variables|Character|GetCharacterMovement))
  (:Pressed
    (Variables|/Script/ProjectFlashpoint.FireComponent|SetbCanFire _fire true)
    (CallFunction|ServerModifyMovementSpeed (* (Variables|/Script/Engine.CharacterMovementComponent|GetMaxWalkSpeed _charactermovement) 0.4))
    (bind (_direction _fov _scopeopacity) (Timeline|FOV%20Timeline Play)
      (:Update
        (Variables|/Script/Engine.CameraComponent|SetFieldOfView (Variables|Default|GetfirstPersonCameraComponent) _fov)
        (bind _output_get (Variables|/Game/Dynamic/Game/BaseGame/PlayerHUD.PlayerHUD_C|SetScopeOpacity (.AsPlayer%20HUD (Utilities|Casting|CastToPlayerHUD (HUD|GetHUD (Game|GetPlayerController 0)))) _scopeopacity))
        (Development|PrintString (Utilities|String|ToString(Float) _output_get)))))
  (:Released
    (Variables|/Script/ProjectFlashpoint.FireComponent|SetbCanFire _fire false)
    (CallFunction|ServerModifyMovementSpeed (* (Variables|/Script/Engine.CharacterMovementComponent|GetMaxWalkSpeed _charactermovement) 2.5))
    (Timeline|FOV%20Timeline Reverse)))

(fn ConstructionScript
  (|CallParentFunction))