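; Smokescreen is a soldier Blueprint whose ability is throwing a smoke grenade.
; Its construction script adds a grenade component set to the SmokeGrenade class with a timed fuse and stores it as the Ability.
; The component gets limited ammo and reserves and is attached to the first-person camera at an offset.
; The event graph holds only disabled placeholder events.
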(event EventBeginPlay
  (|CallParentFunction) ; This node is disabled and will not be called.\nDrag off pins to build functionality.
)

(event Collision|EventActorBeginOverlap
  (params (OtherActor :type Actor%20Object%20Reference)))

(event EventTick
  (params (DeltaSeconds :type Float%20%28single-precision%29))
  (|CallParentFunction DeltaSeconds) ; This node is disabled and will not be called.\nDrag off pins to build functionality.
)

(fn ConstructionScript
  (bind _returnvalue (AddComponent|AddGrenadeComponent false (Math|Transform|MakeTransform "40.000000,15.000000,60.000000" "7.500000, 0,0.000000") "/Game/Dynamic/Abilities/SmokeGrenade.SmokeGrenade_C" 4.0))
  (bind _output_get (Variables|Default|SetAbility _returnvalue))
  (Variables|/Game/Dynamic/Abilities/BaseAbility.BaseAbility_C|SetAmmo _output_get 1)
  (Variables|/Game/Dynamic/Abilities/BaseAbility.BaseAbility_C|SetReserves _output_get 1)
  (Transformation|AttachComponentToComponent _output_get (Variables|Default|GetfirstPersonCameraComponent) "None" "KeepRelative" "KeepRelative" "KeepRelative" true))