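; Base player-controlled soldier character handling look, jog, crouch, prone, jump, aim and weapon input.
; Stance inputs set mutually gated state flags and switch walk speed, with crouch and prone as toggles, while jump height depends on whether the soldier is moving.
; Fire, reload and fire-mode inputs delegate to Fire, whose magazine count is pushed to an AmmoDisplay widget every Tick.
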(event EventBeginPlay
  ;[1 1 1] Begin Play
  (Utilities|FlowControl|Sequence
    (:then_0
      (Variables|/Script/Engine.CharacterMovementComponent|SetMaxWalkSpeed (Variables|Character|GetCharacterMovement) (Variables|Default|GetwalkSpeed)))
    (:then_1
      (CallFunction|ShowWidget))))

(event EventTick
  (params (DeltaSeconds :type Float%20%28single-precision%29))
  (CallFunction|ShowWidget))

(event EventPossessed
  (params (NewController :type Controller%20Object%20Reference))
  (bind _asplayer_controller (Utilities|Casting|CastToPlayerController (Pawn|GetController)))
  (Variables|/Script/Engine.PlayerController|SetbShowMouseCursor _asplayer_controller false))

(event Input|ActionEvents|InputActionWeaponMode
  (params (Key :type Key%20Structure))
  (:Pressed
    (Class|FireComponent|ToggleFireMode (Variables|Default|GetFire))))

(event Input|ActionEvents|InputActionCrouch
  (params (Key :type Key%20Structure))
  (bind _charactermovement (Variables|Character|GetCharacterMovement))
  ;[1 1 1] Crouch
  (:Pressed
    (if (not (Variables|Default|GetPronePressed))
      (Utilities|FlowControl|FlipFlop
        (:A
          (Variables|Default|SetJogPressed false)
          (Variables|Default|SetCrouchPressed true)
          (Variables|/Script/Engine.CharacterMovementComponent|SetMaxWalkSpeed _charactermovement (Variables|Default|GetCrouchSpeed)))
        (:B
          (Variables|Default|SetCrouchPressed false)
          (Variables|/Script/Engine.CharacterMovementComponent|SetMaxWalkSpeed _charactermovement (Variables|Default|GetwalkSpeed)))))))

(event Input|ActionEvents|InputActionJump
  (params (Key :type Key%20Structure))
  (bind _charactermovement (Variables|Character|GetCharacterMovement))
  ;[1 1 1] Jump Based on Velocity
  (:Pressed
    (if (not (Variables|Default|GetAimPressed))
      (if (not (Variables|Default|GetDisableMovement))
        (if (Variables|Default|GetCrouchPressed)
          (if (> (Variables|/Script/Engine.CharacterMovementComponent|GetMaxWalkSpeed (Variables|Character|GetCharacterMovement)) (Variables|Default|GetwalkSpeed))
            (if (> (Math|Vector|VectorLength (Variables|/Script/Engine.MovementComponent|GetVelocity (Variables|Character|GetCharacterMovement))) 0.0) :!label _label
              (Character|Jump)
              (Variables|/Script/Engine.CharacterMovementComponent|SetJumpZVelocity _charactermovement 365.0)
              (Variables|Default|SetJumpPressed true)
              (else
                (Character|Jump)
                (Variables|/Script/Engine.CharacterMovementComponent|SetJumpZVelocity _charactermovement 3.4e+02)
                (Variables|Default|SetJumpPressed true))))
          (else
            (goto _label))))))
  (:Released
    (Variables|Default|SetJumpPressed false)))

(event Input|ActionEvents|InputActionSprint
  (params (Key :type Key%20Structure))
  (bind _charactermovement (Variables|Character|GetCharacterMovement))
  ;[1 1 1] Jog
  (:Pressed
    (if (not (or (Variables|Default|GetCrouchPressed) (Variables|Default|GetPronePressed)))
      (Variables|Default|SetJogPressed true)
      (Variables|/Script/Engine.CharacterMovementComponent|SetMaxWalkSpeed _charactermovement (Variables|Default|GetjogSpeed))))
  (:Released
    (if (Variables|Default|GetJogPressed)
      (Variables|Default|SetJogPressed false)
      (Variables|/Script/Engine.CharacterMovementComponent|SetMaxWalkSpeed _charactermovement (Variables|Default|GetwalkSpeed)))))

(event Input|ActionEvents|InputActionAim
  (params (Key :type Key%20Structure))
  ;[1 1 1] Aim
  (:Pressed
    (if (not (Variables|Default|GetJogPressed))
      (Variables|Default|SetAimPressed true)))
  (:Released
    (Variables|Default|SetAimPressed false)))

(event Input|ActionEvents|InputActionProne
  (params (Key :type Key%20Structure))
  (bind _charactermovement (Variables|Character|GetCharacterMovement))
  ;[1 1 1] Prone
  (:Pressed
    (if (not (or (Variables|Default|GetCrouchPressed) (Variables|Default|GetJogPressed)))
      (Utilities|FlowControl|FlipFlop
        (:A
          (Variables|Default|SetPronePressed true)
          (Variables|/Script/Engine.CharacterMovementComponent|SetMaxWalkSpeed _charactermovement (Variables|Default|GetproneSpeed)))
        (:B
          (Variables|Default|SetPronePressed false)
          (Utilities|FlowControl|Delay 1.4)
          (Variables|/Script/Engine.CharacterMovementComponent|SetMaxWalkSpeed _charactermovement (Variables|Default|GetwalkSpeed)))))))

(event Input|ActionEvents|InputActionFire
  (params (Key :type Key%20Structure))
  (bind _fire (Variables|Default|GetFire))
  ;[1 1 1] Shooting
  (:Pressed
    (Variables|Default|SetShooting true)
    (Class|FireComponent|OnFire _fire))
  (:Released
    (Variables|Default|SetShooting false)
    (Class|FireComponent|OnRelease _fire)))

(event Input|ActionEvents|InputActionReload
  (params (Key :type Key%20Structure))
  (bind _fire (Variables|Default|GetFire))
  ;[1 1 1] Reload
  (:Pressed
    (Variables|Default|SetReloading true)
    (Class|FireComponent|OnReload _fire))
  (:Released
    (Variables|Default|SetReloading false)
    (Class|FireComponent|OnReload _fire)))

(event Input|AxisEvents|InputAxisTurn
  (params (AxisValue :type Float%20%28single-precision%29))
  ;[1 1 1] Aim
  (Pawn|Input|AddControllerYawInput AxisValue))

(event Input|AxisEvents|InputAxisLookUp
  (params (AxisValue :type Float%20%28single-precision%29))
  (bind _charactermovement (Variables|Character|GetCharacterMovement))
  (bind _returnvalue (Class|CharacterMovementComponent|GetCharacterOwner _charactermovement))
  (bind _returnvalue_2 (Pawn|GetControlRotation _returnvalue :!class /Script/Engine.Pawn))
  (bind _pitch (Math|Rotator|BreakRotator _returnvalue_2))
  ;[1 1 1] Aim
  (Pawn|Input|AddControllerPitchInput AxisValue)
  (if (> _pitch 1.8e+02)
    (Variables|Default|SetPitch (- _pitch 3.6e+02))
    (else
      (Variables|Default|SetPitch _pitch))))

(fn ConstructionScript)

(fn ShowWidget
  (bind _asammo_display (Utilities|Casting|CastToAmmoDisplay (UserInterface|GetUserWidgetObject (Variables|Default|GetWidget)))
    (:then
      (bind _output_get (Variables|Default|SetAmmoRef _asammo_display))
      (Rendering|Components|TextRender|SetText (Variables|/Game/Dynamic/Soldiers/Blueprints/AmmoDisplay.AmmoDisplay_C|GetAmmoCount _output_get) (Utilities|Text|ToText(Integer) (Class|FireComponent|GetCurrentMagazineSize (Variables|Default|GetFire)))))
    (:CastFailed
      (Development|PrintString "CastFailed"))))