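; Sniper soldier character Blueprint that adds aim-down-sights zoom with slowed movement.
; Holding Aim plays a timeline that drives the first-person camera's field of view, and releasing reverses it.
; Walk speed is scaled down and back up by reciprocal multipliers of its current value, passed through Server-to-Multicast events that set it on the movement component.
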(event Custom|Server%20Modify%20Movement%20Speed
  (params (newSpeed :type Float%20%28single-precision%29))
  (CallFunction|MulticastModifyMovementSpeed newSpeed))

(event Custom|Multicast%20Modify%20Movement%20Speed
  (params (newSpeed :type Float%20%28single-precision%29))
  (Variables|/Script/Engine.CharacterMovementComponent|SetMaxWalkSpeed (Variables|Character|GetCharacterMovement) newSpeed))

(event EventBeginPlay
  (|CallParentFunction) ; This node is disabled and will not be called.\nDrag off pins to build functionality.
)

(event Collision|EventActorBeginOverlap
  (params (OtherActor :type Actor%20Object%20Reference)))

(event EventTick
  (params (DeltaSeconds :type Float%20%28single-precision%29))
  (|CallParentFunction DeltaSeconds) ; This node is disabled and will not be called.\nDrag off pins to build functionality.
)

(event Input|ActionEvents|InputActionAim
  (params (Key :type Key%20Structure))
  (bind _charactermovement (Variables|Character|GetCharacterMovement))
  (:Pressed
    (CallFunction|ServerModifyMovementSpeed (* (Variables|/Script/Engine.CharacterMovementComponent|GetMaxWalkSpeed _charactermovement) 0.4))
    (bind _fov (Timeline|Timeline_0 Play)
      (:Update
        (Variables|/Script/Engine.CameraComponent|SetFieldOfView (Variables|Default|GetfirstPersonCameraComponent) _fov))))
  (:Released
    (CallFunction|ServerModifyMovementSpeed (* (Variables|/Script/Engine.CharacterMovementComponent|GetMaxWalkSpeed _charactermovement) 2.5))
    (Timeline|Timeline_0 Reverse)))

(fn ConstructionScript
  (|CallParentFunction))