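; HotLead is a soldier-related Blueprint that gates firing and sets recoil according to the current action state.
; Every Tick, it reads the action state from GetActionState and writes to its Fire member.
; Some states block firing, while two allow it with different vertical and horizontal recoil profiles, one much tighter than the other.
; All other behavior comes from the parent class.
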(event EventBeginPlay
  (|CallParentFunction) ; This node is disabled and will not be called.\nDrag off pins to build functionality.
)

(event Collision|EventActorBeginOverlap
  (params (OtherActor :type Actor%20Object%20Reference)))

(event EventTick
  (params (DeltaSeconds :type Float%20%28single-precision%29))
  (bind _fire (Variables|Default|GetFire))
  (bind _fire_2 (Variables|Default|GetFire))
  (|CallParentFunction DeltaSeconds)
  (bind _returnvalue (Class|Soldier|GetActionState))
  (switch int _returnvalue
    (:1
      (Variables|/Script/ProjectFlashpoint.FireComponent|SetbCanFire _fire false :!label _label))
    (:2
      (goto _label))
    (:3
      (Variables|/Script/ProjectFlashpoint.FireComponent|SetbCanFire _fire true)
      (Variables|/Script/ProjectFlashpoint.FireComponent|SetverticalRecoil _fire_2 0.1)
      (Variables|/Script/ProjectFlashpoint.FireComponent|SetminVerticalRecoil _fire_2 0.06)
      (Variables|/Script/ProjectFlashpoint.FireComponent|SethorizontalRecoil _fire_2 0.1))
    (:4
      (Variables|/Script/ProjectFlashpoint.FireComponent|SetbCanFire _fire true)
      (Variables|/Script/ProjectFlashpoint.FireComponent|SetverticalRecoil _fire_2 0.04)
      (Variables|/Script/ProjectFlashpoint.FireComponent|SetminVerticalRecoil _fire_2 0.01)
      (Variables|/Script/ProjectFlashpoint.FireComponent|SethorizontalRecoil _fire_2 0.02))
    (:5
      (goto _label))))

(fn ConstructionScript
  (|CallParentFunction))